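; Minimap manager Blueprint that creates Minimap_WB widgets and controls their paths and appearance at runtime.
; An add-minimap event, optionally auto-fired after BeginPlay, creates one for a given player, every PlayerController in split screen, or the viewport.
; Path functions forward named lines to the cached widget, or to all of them in split screen.
; SetMinimapRender changes material parameters, border and canvas layout, or restores defaults, targeting the matching player's widget in split screen.
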(event Custom|AddMinimap_Event
  (params (Specific%20Player :type Player%20Controller%20Object%20Reference))
  ;[1 0.356 0] Seta as configurações iniciais do minimapa
  (Utilities|IsValid Specific%20Player
    (:Is%20Valid
      (bind _returnvalue (UserInterface|CreateWidget "/Game/Minimap/Minimap_WB.Minimap_WB_C" Specific%20Player (Variables|Default|GetMinimapTexture) (Variables|Default|GetMinimapTextureMask) self))
      (UserInterface|Viewport|AddtoPlayerScreen _returnvalue))
    (:Is%20Not%20Valid
      (if (Variables|Default|GetIsSplitScreen)
        (bind _outactors (Actor|GetAllActorsOfClass "/Script/Engine.PlayerController"))
        (for _array_element _outactors
          (bind _returnvalue_2 (UserInterface|CreateWidget "/Game/Minimap/Minimap_WB.Minimap_WB_C" _array_element (Variables|Default|GetMinimapTexture) (Variables|Default|GetMinimapTextureMask) self))
          (UserInterface|Viewport|AddtoPlayerScreen _returnvalue_2))
        (else
          (bind _returnvalue_3 (UserInterface|CreateWidget "/Game/Minimap/Minimap_WB.Minimap_WB_C" 0 (Variables|Default|GetMinimapTexture) (Variables|Default|GetMinimapTextureMask) self))
          (bind _output_get (Variables|Default|SetMinimap_W _returnvalue_3))
          (UserInterface|Viewport|AddtoViewport _output_get 0))))))

(event EventBeginPlay
  ;[1 0.356 0] Seta as configurações iniciais do minimapa
  (EventDispatchers|BindEventtoAddMinimap (delegate Custom|AddMinimap_Event))
  (Variables|Default|SetDefaultSize (Variables|Default|GetMinimapSize))
  (Variables|Default|SetDefaultIsSpherica (Variables|Default|GetIsSphericalMap))
  (Variables|Default|SetDefaultGPS_Mode (Variables|Default|GetGPS_Mode))
  (if (Variables|Default|GetAutoCreateMinimap)
    (Utilities|FlowControl|Delay 0.03)
    (Default|CallAddMinimap)))

(fn ConstructionScript)

(fn FindMinimapPlayer
  (params (Player :type Player%20Controller%20Object%20Reference))
  (bind _foundwidgets (Widget|GetAllWidgetsOfClass "/Game/Minimap/Minimap_WB.Minimap_WB_C" true))
  (for _array_element _foundwidgets
    (if (== Player (Widget|GetOwningPlayer _array_element))
      (bind _asminimap_wb (Utilities|Casting|CastToMinimap_WB _array_element))
      (return _asminimap_wb)))
  (return 0))

(fn DrawPathLine
  (params (Points :type Array%20of%20Vectors) (Name :type String) (Color :type Linear%20Color%20Structure) (Width :type Float%20%28single-precision%29) (Gradient :type Float%20%28single-precision%29))
  (bind _output_get (LocalVariables|SetLocalPoints Points))
  (if (Variables|Default|GetIsSplitScreen)
    (bind _foundwidgets (Widget|GetAllWidgetsOfClass "/Game/Minimap/Minimap_WB.Minimap_WB_C" true))
    (for _array_element _foundwidgets
      (bind _asminimap_wb (Utilities|Casting|CastToMinimap_WB _array_element))
      (Default|DrawPath _asminimap_wb _output_get Name Color Width Gradient))
    (else
      (bind _minimap_w (Variables|Default|GetMinimap_W)
        (:then
          (Default|DrawPath _minimap_w _output_get Name Color Width Gradient))
        (:else)))))

(fn DestroyPathLine
  (params (Name :type String))
  (if (Variables|Default|GetIsSplitScreen)
    (bind _foundwidgets (Widget|GetAllWidgetsOfClass "/Game/Minimap/Minimap_WB.Minimap_WB_C" true))
    (for _array_element _foundwidgets
      (bind _asminimap_wb (Utilities|Casting|CastToMinimap_WB _array_element))
      (Default|DestroyPath _asminimap_wb Name))
    (else
      (bind _minimap_w (Variables|Default|GetMinimap_W)
        (:then
          (Default|DestroyPath _minimap_w Name))
        (:else)))))

(fn SetMinimapRender
  (params (Reset :type Boolean) (PlayerController :type Player%20Controller%20Object%20Reference) (Texture :type Texture%202D%20Object%20Reference) (Mask :type Texture%202D%20Object%20Reference) (BorderTexture :type Texture%202D%20Object%20Reference) (BorderRotation :type Float%20%28single-precision%29) (Anchors :type Anchors%20Structure) (Position :type Vector%202D%20Structure) (Size :type Float%20%28single-precision%29) (IsSphericalMap :type Boolean) (GPS_Mode :type Boolean))
  (bind _minimap_w (Variables|Default|GetMinimap_W))
  (if (Variables|Default|GetIsSplitScreen)
    (bind _foundwidgets (Widget|GetAllWidgetsOfClass "/Game/Minimap/Minimap_WB.Minimap_WB_C" true))
    (for _array_element _foundwidgets
      (if (== (Widget|GetOwningPlayer _array_element) PlayerController)
        (bind _asminimap_wb (Utilities|Casting|CastToMinimap_WB _array_element))
        (if Reset
          (CallFunction|ResetRender _asminimap_wb)
          (else
            (CallFunction|SetRender _asminimap_wb Texture Mask BorderTexture BorderRotation Anchors Position Size IsSphericalMap GPS_Mode)))))
    (elif Reset
      (CallFunction|ResetRender _minimap_w)
      (else
        (CallFunction|SetRender _minimap_w Texture Mask BorderTexture BorderRotation Anchors Position Size IsSphericalMap GPS_Mode)))))

(fn SetRender
  (params (Widget :type Minimap%20WB%20Object%20Reference) (Texture :type Texture%202D%20Object%20Reference) (Mask :type Texture%202D%20Object%20Reference) (BorderTexture :type Texture%202D%20Object%20Reference) (BorderRotation :type Float%20%28single-precision%29) (Anchors :type Anchors%20Structure) (Position :type Vector%202D%20Structure) (Size :type Float%20%28single-precision%29) (IsSphericalMap :type Boolean) (GPS_Mode :type Boolean))
  (bind _returnvalue (Utilities|IsValid BorderTexture))
  (bind _minimappanel (Variables|/Game/Minimap/Minimap_WB.Minimap_WB_C|GetMinimapPanel Widget))
  (bind _minimap_m (Variables|/Game/Minimap/Minimap_WB.Minimap_WB_C|GetMinimap_M Widget))
  (bind _minimapborder (Variables|/Game/Minimap/Minimap_WB.Minimap_WB_C|GetMinimapBorder Widget))
  (bind _minimap_m_2 (Variables|/Game/Minimap/Minimap_WB.Minimap_WB_C|GetMinimap_M Widget))
  (bind _returnvalue_2 (Class|WidgetLayoutLibrary|SlotasCanvasSlot _minimappanel))
  (Variables|Default|SetIsSphericalMap IsSphericalMap)
  (bind _output_get (Variables|Default|SetGPS_Mode GPS_Mode))
  (if _output_get
    _
    (else
      (Rendering|Material|SetScalarParameterValue _minimap_m_2 "Rotation" 0.0 :!class /Script/Engine.MaterialInstanceDynamic)
      (Rendering|Material|SetScalarParameterValue _minimap_m_2 "Size" 1.0 :!class /Script/Engine.MaterialInstanceDynamic)
      (Rendering|Material|SetScalarParameterValue _minimap_m_2 "PosX" 0.0 :!class /Script/Engine.MaterialInstanceDynamic)
      (Rendering|Material|SetScalarParameterValue _minimap_m_2 "PosY" 0.0 :!class /Script/Engine.MaterialInstanceDynamic)))
  (if (Utilities|IsValid Texture)
    (Rendering|Material|SetTextureParameterValue _minimap_m "Texture" Texture))
  (Rendering|Material|SetTextureParameterValue _minimap_m "Mask" Mask)
  (Widget|SetVisibility _minimapborder (select _returnvalue "HitTestInvisible" "Hidden"))
  (if _returnvalue
    (Appearance|SetBrushfromTexture _minimapborder BorderTexture false)
    (Class|Widget|SetRenderAngle _minimapborder BorderRotation))
  (Class|CanvasPanelSlot|SetAnchors _returnvalue_2 Anchors)
  (Class|CanvasPanelSlot|SetPosition _returnvalue_2 Position)
  (Class|CanvasPanelSlot|SetSize _returnvalue_2 (* "(X=1.000000,Y=1.000000)" Size))
  (Variables|Default|SetMinimapSize Size))

(fn ResetRender
  (params (Widget :type Minimap%20WB%20Object%20Reference))
  (CallFunction|SetRender Widget (Variables|Default|GetMinimapTexture) (Variables|Default|GetMinimapTextureMask) (Variables|Default|GetMinimapBorderTexture) (Variables|Default|GetMinimapBorderRotation) (Variables|Default|GetMinimapAnchors) (Variables|Default|GetMinimapScreenPos) (Variables|Default|GetDefaultSize) false false)
  (Variables|Default|SetIsSphericalMap (Variables|Default|GetDefaultIsSpherica))
  (Variables|Default|SetGPS_Mode (Variables|Default|GetDefaultGPS_Mode))
  (Rendering|Material|SetScalarParameterValue (Variables|/Game/Minimap/Minimap_WB.Minimap_WB_C|GetMinimap_M Widget) "Size" (Variables|/Game/Minimap/Minimap_WB.Minimap_WB_C|GetCurrentZoom Widget) :!class /Script/Engine.MaterialInstanceDynamic))