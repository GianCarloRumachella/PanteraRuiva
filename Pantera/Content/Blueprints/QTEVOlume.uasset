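; QTE trigger volume that freezes the Pantera character on box overlap until it completes a key-press quick-time event.
; Overlap shuffles the character's keys, shows the current one in a QTE widget and flags the character as in QTE.
; A per-frame Delay loop updates the progress bar and polls the success flag.
; Success restores walking, removes the widget and temporarily hides the actor; ending overlap also clears widget and QTE flag.
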(event OnComponentBeginOverlap(Box)
  (params (OverlappedComponent :type Primitive%20Component%20Object%20Reference) (OtherActor :type Actor%20Object%20Reference) (OtherComp :type Primitive%20Component%20Object%20Reference) (OtherBodyIndex :type Integer) (bFromSweep :type Boolean) (SweepResult :type Hit%20Result%20Structure%20%28by%20ref%29))
  (bind _aspantera (Utilities|Casting|CastToPantera OtherActor))
  (bind _returnvalue (UserInterface|CreateWidget "/Game/HUD/QTEWidget.QTEWidget_C"))
  (bind _output_get (Variables|Default|Setwidget _returnvalue))
  (UserInterface|Viewport|AddtoViewport _output_get 0)
  (Pawn|Components|CharacterMovement|DisableMovement (Variables|/Script/Engine.Character|GetCharacterMovement _aspantera))
  (Default|ShufleKeys _aspantera)
  (Rendering|Components|TextRender|SetText (Variables|/Game/HUD/QTEWidget.QTEWidget_C|GetKeyText _output_get) (Class|KismetInputLibrary|KeyGetDisplayName (Variables|/Game/Blueprints/Pantera.Pantera_C|GetCurrentKey _aspantera)))
  (Variables|/Game/Blueprints/Pantera.Pantera_C|SetInQTE _aspantera true)
  (Default|UpdateProgressBar (Variables|Default|Getwidget) (Variables|_Tempo|GetTempo) :!label _label)
  (Utilities|FlowControl|Delay (Utilities|Time|GetWorldDeltaSeconds))
  (if (Variables|/Game/Blueprints/Pantera.Pantera_C|GetSucesso _aspantera)
    (Pawn|Components|CharacterMovement|SetMovementMode (Variables|/Script/Engine.Character|GetCharacterMovement _aspantera) "MOVE_Walking" 0)
    (Widget|RemovefromParent (Variables|Default|Getwidget))
    (Variables|/Game/Blueprints/Pantera.Pantera_C|SetInQTE _aspantera false)
    (Variables|/Game/Blueprints/Pantera.Pantera_C|SetSucesso _aspantera false)
    (Rendering|SetActorHiddenInGame true)
    (Utilities|FlowControl|Delay (Variables|Default|GetTempoInvisivel))
    (Rendering|SetActorHiddenInGame false)
    (else
      (goto _label))))

(event OnComponentEndOverlap(Box)
  (params (OverlappedComponent :type Primitive%20Component%20Object%20Reference) (OtherActor :type Actor%20Object%20Reference) (OtherComp :type Primitive%20Component%20Object%20Reference) (OtherBodyIndex :type Integer))
  (Widget|RemovefromParent (Variables|Default|Getwidget))
  (bind _aspantera (Utilities|Casting|CastToPantera OtherActor))
  (Variables|/Game/Blueprints/Pantera.Pantera_C|SetInQTE _aspantera false))

(event EventBeginPlay)

(event Collision|EventActorBeginOverlap
  (params (OtherActor :type Actor%20Object%20Reference)))

(event EventTick
  (params (DeltaSeconds :type Float%20%28single-precision%29)))

(fn ConstructionScript)

(fn VisibleAgain
  (Rendering|SetActorHiddenInGame false))