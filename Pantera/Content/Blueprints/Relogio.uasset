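; Relogio is an analog clock actor that shows the current local time with rotating second, minute and hour hands.
; Every Tick reads Now, maps each time unit to a negative roll through MapRangeClamped, and sets each hand's relative rotation.
; The minute and hour hands add fractional offsets from seconds and minutes, though these are positive and so run against the negative sweep.
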(event EventBeginPlay)

(event Collision|EventActorBeginOverlap
  (params (OtherActor :type Actor%20Object%20Reference)))

(event EventTick
  (params (DeltaSeconds :type Float%20%28single-precision%29))
  (bind _returnvalue (Math|DateTime|Now))
  (bind _returnvalue_2 (Math|DateTime|Now))
  (bind _returnvalue_3 (Class|KismetMathLibrary|GetSecond _returnvalue))
  (bind _returnvalue_4 (Class|KismetMathLibrary|GetMinute _returnvalue_2))
  (bind _returnvalue_5 (Math|Conversions|ToFloat(Integer) _returnvalue_3))
  (bind _returnvalue_6 (Math|Conversions|ToFloat(Integer) _returnvalue_4))
  (Transformation|SetRelativeRotation (Variables|Default|GetPonteiroSegundos) (Math|Rotator|MakeRotator (Math|Float|MapRangeClamped _returnvalue_5 0.0 6e+01 0.0 -3.6e+02) 0.0 0.0) false false)
  (Transformation|SetRelativeRotation (Variables|Default|GetPonteiroMinutos) (Math|Rotator|MakeRotator (+ (Math|Float|MapRangeClamped _returnvalue_6 0.0 6e+01 0.0 -3.6e+02) (/ _returnvalue_5 1e+01)) 0.0 0.0) false false)
  (Transformation|SetRelativeRotation (Variables|Default|GetPonteiroHoras) (Math|Rotator|MakeRotator (+ (Math|Float|MapRangeClamped (Math|Conversions|ToFloat(Integer) (Class|KismetMathLibrary|GetHour12 (Math|DateTime|Now))) 0.0 12.0 0.0 -3.6e+02) (Math|Float|MapRangeClamped _returnvalue_6 0.0 6e+01 0.0 3e+01)) 0.0 0.0) false false))

(fn ConstructionScript)