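; SmashButtonVolume is a trigger volume that starts a button-smash prompt when the Pantera character enters its box.
; BeginPlay caches the PanteraGame game mode and disables the actor's collision.
; On overlap it changes Pantera's action state, shows an SBWidget displaying a key from the game mode's ShuffleKeys, and calls FullProgressBar.
; The end-overlap event is empty, leaving the widget-removal logic disconnected.
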(event OnComponentBeginOverlap(Box)
  (params (OverlappedComponent :type Primitive%20Component%20Object%20Reference) (OtherActor :type Actor%20Object%20Reference) (OtherComp :type Primitive%20Component%20Object%20Reference) (OtherBodyIndex :type Integer) (bFromSweep :type Boolean) (SweepResult :type Hit%20Result%20Structure%20%28by%20ref%29))
  (bind _aspantera (Utilities|Casting|CastToPantera OtherActor))
  (Variables|/Game/Blueprints/Pantera.Pantera_C|SetActions _aspantera "NewEnumerator1")
  (bind _returnvalue (UserInterface|CreateWidget "/Game/HUD/SBWidget.SBWidget_C"))
  (bind _output_get (Variables|/Game/Blueprints/Pantera.Pantera_C|SetW_SmashButton _aspantera _returnvalue))
  (UserInterface|Viewport|AddtoViewport _output_get 0)
  (bind _output_get_2 (Variables|/Game/Blueprints/Pantera.Pantera_C|SetCurrentKey _aspantera (Default|ShuffleKeys (Variables|Default|GetGM))))
  (Rendering|Components|TextRender|SetText (Variables|/Game/HUD/SBWidget.SBWidget_C|GetSBKey _output_get) (Class|KismetInputLibrary|KeyGetDisplayName _output_get_2))
  (Default|FullProgressBar _aspantera))

(event OnComponentEndOverlap(Box)
  (params (OverlappedComponent :type Primitive%20Component%20Object%20Reference) (OtherActor :type Actor%20Object%20Reference) (OtherComp :type Primitive%20Component%20Object%20Reference) (OtherBodyIndex :type Integer)))

(event EventBeginPlay
  (bind _aspantera_game (Utilities|Casting|CastToPanteraGame (Game|GetGameMode)))
  (Variables|Default|SetGM _aspantera_game)
  (Collision|SetActorEnableCollision false))

(fn ConstructionScript)