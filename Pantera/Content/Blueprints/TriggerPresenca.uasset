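; TriggerPresenca is a one-shot trigger volume that reacts when the Pantera character enters its Box component.
; On overlap it sets the EActions state on the PanteraGame game mode and disables the Pantera's character movement.
; It then turns off its own collision and hides itself, so it stops responding to further overlaps.
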(event OnComponentBeginOverlap(Box)
  (params (OverlappedComponent :type Primitive%20Component%20Object%20Reference) (OtherActor :type Actor%20Object%20Reference) (OtherComp :type Primitive%20Component%20Object%20Reference) (OtherBodyIndex :type Integer) (bFromSweep :type Boolean) (SweepResult :type Hit%20Result%20Structure%20%28by%20ref%29))
  (if (== (Utilities|GetClass OtherActor) "/Game/Blueprints/Pantera.Pantera_C")
    (bind _aspantera_game (Utilities|Casting|CastToPanteraGame (Game|GetGameMode)))
    (Variables|/Game/Blueprints/PanteraGame.PanteraGame_C|SetE_Actions _aspantera_game "NewEnumerator3")
    (bind _aspantera (Utilities|Casting|CastToPantera OtherActor))
    (Pawn|Components|CharacterMovement|DisableMovement (Variables|/Script/Engine.Character|GetCharacterMovement _aspantera))
    (Collision|SetActorEnableCollision false)
    (Rendering|SetActorHiddenInGame true)))

(event EventBeginPlay)

(event Collision|EventActorBeginOverlap
  (params (OtherActor :type Actor%20Object%20Reference)))

(event EventTick
  (params (DeltaSeconds :type Float%20%28single-precision%29)))

(fn ConstructionScript)