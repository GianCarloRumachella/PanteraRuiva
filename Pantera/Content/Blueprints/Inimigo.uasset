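; Enemy actor (Inimigo) that loops the Espadada animation and sequences trigger stages through the PanteraGame game mode's EActions state.
; Tick switches on that state: Presence immediately hides its trigger and becomes QTE, which advances to SmashButton once Sucesso is true, hiding the QTE trigger.
; The QTE and SmashButton stages each enable collision on their child-actor volume every tick they are active.
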(event EventBeginPlay
  (bind _aspantera_game (Utilities|Casting|CastToPanteraGame (Game|GetGameMode)))
  (Variables|Default|SetPanteraGM _aspantera_game)
  (Components|Animation|PlayAnimation (Variables|Character|GetMesh) "/Game/Mannequin/Animations/Espadada.Espadada" true))

(event EventTick
  (params (DeltaSeconds :type Float%20%28single-precision%29))
  (bind _triggerqte (Variables|Default|GetTriggerQTE))
  (bind _panteragm (Variables|Default|GetPanteraGM)
    (:then
      (switch Utilities|FlowControl|Switch|SwitchonEActions (Variables|/Game/Blueprints/PanteraGame.PanteraGame_C|GetE_Actions _panteragm)
        (:NewEnumerator3
          (Variables|/Game/Blueprints/PanteraGame.PanteraGame_C|SetE_Actions (Variables|Default|GetPanteraGM) "NewEnumerator0")
          (Development|SetHiddeninGame (Variables|Default|GetTriggerPresenca) true false))
        (:NewEnumerator0
          (bind _asqtevolume (Utilities|Casting|CastToQTEVOlume (Variables|/Script/Engine.ChildActorComponent|GetChildActor _triggerqte)))
          (Collision|SetActorEnableCollision _asqtevolume true)
          (if (Variables|Default|GetSucesso)
            (Variables|/Game/Blueprints/PanteraGame.PanteraGame_C|SetE_Actions (Variables|Default|GetPanteraGM) "NewEnumerator1")
            (Development|SetHiddeninGame _triggerqte true false)))
        (:NewEnumerator1
          (bind _assmash_button_volume (Utilities|Casting|CastToSmashButtonVolume (Variables|/Script/Engine.ChildActorComponent|GetChildActor (Variables|Default|GetTriggerSmash))))
          (Collision|SetActorEnableCollision _assmash_button_volume true))))
    (:else)))

(fn ConstructionScript)